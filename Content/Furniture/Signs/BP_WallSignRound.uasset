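; BP_WallSignRound is a furniture wall sign that randomizes its look on BeginPlay.
; It picks a coffee cup, shing or bistro mesh at roughly equal odds, adjusting the mesh transform as needed and repositioning BPText2D to suit each shape.
; It then tints the sign with a random color through the Albedo_1_ColorOverlay material parameter.
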(event EventBeginPlay
  (bind _sm_signs_sign_antiques (Variables|Default|GetSM_signs_sign_antiques))
  (bind _bp_text2d (Variables|Default|GetBP_Text2D))
  (if (> (Math|Random|RandomFloat) 0.666)
    (Components|StaticMesh|SetStaticMesh _sm_signs_sign_antiques "/Game/Furniture/Signs/Mesh/SM_signs_sign_coffeecup.SM_signs_sign_coffeecup")
    (Transformation|SetRelativeLocation _bp_text2d "48.000000,3.800000,-13.400000" false false)
    (elif (Math|Random|RandomBool)
      (Components|StaticMesh|SetStaticMesh _sm_signs_sign_antiques "/Game/Furniture/Signs/Mesh/SM_signs_sign_shing.SM_signs_sign_shing")
      (Transformation|SetRelativeRotation _sm_signs_sign_antiques "0,180.000000, 0" false false)
      (Transformation|SetRelativeLocation _bp_text2d "61.000000,3.800000,-13.400000" false false)
      (else
        (Components|StaticMesh|SetStaticMesh _sm_signs_sign_antiques "/Game/Furniture/Signs/Mesh/SM_signs_sign_bistro.SM_signs_sign_bistro")
        (Transformation|SetRelativeRotation _sm_signs_sign_antiques "0,180.000000, 0" false false)
        (Transformation|SetRelativeLocation _sm_signs_sign_antiques "0, 0,20.000000" false false)
        (Transformation|SetRelativeLocation _bp_text2d "61.000000,3.800000,-40.000000" false false))))
  (Rendering|Material|SetVectorParameterValueonMaterials _sm_signs_sign_antiques "Albedo_1_ColorOverlay" (Math|Vector|MakeVector (Math|Random|RandomFloat) (Math|Random|RandomFloat) (Math|Random|RandomFloat))))

(event Collision|EventActorBeginOverlap
  (params (OtherActor :type Actor%20Object%20Reference)))

(event EventTick
  (params (DeltaSeconds :type Float%20%28single-precision%29)))

(fn ConstructionScript)