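; BP_WallSignLarge is a furniture prop for a large wall sign that randomizes its look at runtime.
; On BeginPlay it randomly swaps its static mesh among deli, Bhive and antiques variants, each roughly equally likely.
; It then tints the sign by setting a random RGB color overlay parameter on the mesh's materials.
; The construction script is empty, so the variation appears only once play starts.
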(event EventBeginPlay
  (bind _sm_signs_sign_antiques (Variables|Default|GetSM_signs_sign_antiques))
  (if (> (Math|Random|RandomFloat) 0.666)
    (Components|StaticMesh|SetStaticMesh _sm_signs_sign_antiques "/Game/Furniture/Signs/Mesh/SM_signs_sign_deli.SM_signs_sign_deli")
    (elif (Math|Random|RandomBool)
      (Components|StaticMesh|SetStaticMesh _sm_signs_sign_antiques "/Game/Furniture/Signs/Mesh/SM_signs_sign_Bhive.SM_signs_sign_Bhive")
      (else
        (Components|StaticMesh|SetStaticMesh _sm_signs_sign_antiques "/Game/Furniture/Signs/Mesh/SM_signs_sign_antiques.SM_signs_sign_antiques"))))
  (Rendering|Material|SetVectorParameterValueonMaterials _sm_signs_sign_antiques "Albedo_1_ColorOverlay" (Math|Vector|MakeVector (Math|Random|RandomFloat) (Math|Random|RandomFloat) (Math|Random|RandomFloat))))

(event Collision|EventActorBeginOverlap
  (params (OtherActor :type Actor%20Object%20Reference)))

(event EventTick
  (params (DeltaSeconds :type Float%20%28single-precision%29)))

(fn ConstructionScript)