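; BP_RoomGrid is a placer actor that fills a grid with randomized rooms when play begins.
; On BeginPlay, a 2D grid macro lays out cells around the actor's location from its sector counts and spacing.
; Each cell spawns a BP_RandomRoom at its center with a random yaw in 90-degree steps.
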(event EventBeginPlay
  (bind _poly_center (Utilities|2DGridExecutionMacro (Variables|Default|GetSpacing) (Transformation|GetActorLocation) (Variables|Default|GetSectorX) (Variables|Default|GetSectorY))
    (:Per%20Poly%20Execution
      (Game|SpawnActorfromClass "/Game/Furniture/Rooms/Mesh/BP_RandomRoom.BP_RandomRoom_C" (Math|Transform|MakeTransform (Math|Vector|MakeVector (.x _poly_center) (.y _poly_center) (.z _poly_center)) (Math|Rotator|MakeRotator 0.0 0.0 (Math|Conversions|ToFloat(Integer) (* 90 (Math|Random|RandomIntegerinRange 0 3)))) "1,1,1") "Undefined" 0 0))))

(event Collision|EventActorBeginOverlap
  (params (OtherActor :type Actor%20Object%20Reference)))

(event EventTick
  (params (DeltaSeconds :type Float%20%28single-precision%29)))

(fn ConstructionScript)