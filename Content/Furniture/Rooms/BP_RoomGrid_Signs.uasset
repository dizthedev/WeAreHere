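; BP_RoomGrid_Signs is a grid spawner that lays out room target actors around its own location at game start.
; After a short delay, a 2D grid macro spawns a BP_RoomTarget at each cell center, using the spacing and sector-count variables.
; Disconnected leftovers include spawning randomly quarter-turned BP_RandomRoom_Signs rooms, player position checks and delayed room cleanup, none of which run.
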(event Custom|PlayerLocation
  (Actor|GetAllActorsOfClass "/Game/Furniture/Rooms/BP_RoomTarget.BP_RoomTarget_C"))

(event Custom|BeginPlayerPosition)

(event EventBeginPlay
  (Utilities|FlowControl|Delay 0.2)
  (bind _poly_center (Utilities|2DGridExecutionMacro (Variables|Default|GetSpacing) (Transformation|GetActorLocation) (Variables|Default|GetSectorX_0) (Variables|Default|GetSectorY_0))
    (:Per%20Poly%20Execution
      (bind _returnvalue (Game|SpawnActorfromClass "/Game/Furniture/Rooms/BP_RoomTarget.BP_RoomTarget_C" (Math|Transform|MakeTransform (Math|Vector|MakeVector (.x _poly_center) (.y _poly_center) (.z _poly_center)) (Math|Rotator|MakeRotator 0.0 0.0 0.0) "1,1,1") "Undefined" 0 0))
      (Actor|GetAllActorsOfClass (Utilities|GetClass _returnvalue)))))

(event Collision|EventActorBeginOverlap
  (params (OtherActor :type Actor%20Object%20Reference)))

(event EventTick
  (params (DeltaSeconds :type Float%20%28single-precision%29)))

(fn ConstructionScript)