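; BP_RandomRoom_signs is an actor that randomizes a modular hallway piece when play begins.
; On BeginPlay it sets the class of its BPStraightHall2 child actor to a random pick from hall, intersection, diagonal, dead-end and dead-space Blueprints.
; Unconnected nodes for random static mesh and material selection remain in the graph but never run, and the construction script is empty.
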(event EventBeginPlay
  (ChildActorComponent|SetChildActorClass (Variables|Default|GetBP_StraightHall_2) (.OutItem (Utilities|Array|Random (Utilities|Array|MakeArray "/Game/Furniture/Rooms/Mesh/BP_2WayDiag.BP_2WayDiag_C" "/Game/Furniture/Rooms/Mesh/BP_3Intersect.BP_3Intersect_C" "/Game/Furniture/Rooms/Mesh/BP_3IntersectOpen.BP_3IntersectOpen_C" "/Game/Furniture/Rooms/Mesh/BP_4Intersect.BP_4Intersect_C" "/Game/Furniture/Rooms/Mesh/BP_4IntersectOpen.BP_4IntersectOpen_C" "/Game/Furniture/Rooms/Mesh/BP_StraightHall_2.BP_StraightHall_2_C" "/Game/Furniture/Rooms/Mesh/BP_DeadEnd.BP_DeadEnd_C" "/Game/Furniture/Rooms/Mesh/BP_DeadSpace.BP_DeadSpace_C")))))

(event Collision|EventActorBeginOverlap
  (params (OtherActor :type Actor%20Object%20Reference)))

(event EventTick
  (params (DeltaSeconds :type Float%20%28single-precision%29)))

(fn ConstructionScript)