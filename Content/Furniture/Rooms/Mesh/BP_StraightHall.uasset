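; Straight hallway room Blueprint that populates itself with large wall signs, round wall signs and standing signs at BeginPlay.
; A sequence runs one 2D grid macro per sign type, centered on that type's placed component, with its own spacing and sector counts.
; Each cell spawns a sign actor using the component's yaw, offset one spacing along world Y.
; The random multipliers are all fixed at 1, so layouts are deterministic.
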(event EventBeginPlay
  (Utilities|FlowControl|Sequence
    (:then_0
      (bind _poly_center (Utilities|2DGridExecutionMacro (Variables|Default|GetSpacing) (Transformation|GetWorldLocation (Variables|Default|GetBP_WallSignLarge)) (* (Variables|Default|GetSectorX) (Math|Random|RandomIntegerinRange 1 1)) (* (Variables|Default|GetSectorY) (Math|Random|RandomIntegerinRange 1 1)))
        (:Per%20Poly%20Execution
          (Game|SpawnActorfromClass "/Game/Furniture/Signs/BP_WallSignLarge.BP_WallSignLarge_C" (Math|Transform|MakeTransform (Math|Vector|MakeVector (.x _poly_center) (+ (.y _poly_center) (* (Variables|Default|GetSpacing) (Math|Random|RandomFloatinRange 1.0 1.0))) (.z _poly_center)) (Math|Rotator|MakeRotator 0.0 0.0 (.yaw (Transformation|GetWorldRotation (Variables|Default|GetBP_WallSignLarge)))) "1,1,1") "Undefined" 0 0))))
    (:then_1
      (bind _poly_center_2 (Utilities|2DGridExecutionMacro (Variables|Default|GetSpacing_0) (Transformation|GetWorldLocation (Variables|Default|GetBP_WallSignRound)) (* (Variables|Default|GetSectorX_0) (Math|Random|RandomIntegerinRange 1 1)) (* (Variables|Default|GetSectorY_0) (Math|Random|RandomIntegerinRange 1 1)))
        (:Per%20Poly%20Execution
          (Game|SpawnActorfromClass "/Game/Furniture/Signs/BP_WallSignRound.BP_WallSignRound_C" (Math|Transform|MakeTransform (Math|Vector|MakeVector (.x _poly_center_2) (+ (.y _poly_center_2) (* (Variables|Default|GetSpacing_0) (Math|Random|RandomFloatinRange 1.0 1.0))) (.z _poly_center_2)) (Math|Rotator|MakeRotator 0.0 0.0 (.yaw (Transformation|GetWorldRotation (Variables|Default|GetBP_WallSignRound)))) "1,1,1") "Undefined" 0 0))))
    (:then_2
      (bind _poly_center_3 (Utilities|2DGridExecutionMacro (Variables|Default|GetSpacing_1) (Transformation|GetWorldLocation (Variables|Default|GetBP_StandingSign)) (* (Variables|Default|GetSectorX_1) (Math|Random|RandomIntegerinRange 1 1)) (* (Variables|Default|GetSectorY_1) (Math|Random|RandomIntegerinRange 1 1)))
        (:Per%20Poly%20Execution
          (Game|SpawnActorfromClass "/Game/Furniture/Signs/BP_StandingSign.BP_StandingSign_C" (Math|Transform|MakeTransform (Math|Vector|MakeVector (.x _poly_center_3) (+ (.y _poly_center_3) (* (Variables|Default|GetSpacing_1) (Math|Random|RandomFloatinRange 1.0 1.0))) (.z _poly_center_3)) (Math|Rotator|MakeRotator 0.0 0.0 (.yaw (Transformation|GetWorldRotation (Variables|Default|GetBP_StandingSign)))) "1,1,1") "Undefined" 0 0))))))

(event Collision|EventActorBeginOverlap
  (params (OtherActor :type Actor%20Object%20Reference)))

(event EventTick
  (params (DeltaSeconds :type Float%20%28single-precision%29)))

(fn ConstructionScript)