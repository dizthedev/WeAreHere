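; BP_RoomTarget is a placement point that streams a randomly rotated BP_RandomRoom_Signs actor in and out based on player distance.
; A looping one-second timer measures the distance from the player pawn to its root.
; Inside the range, a Gate lets one room spawn at a random quarter-turn yaw, then closes.
; Outside it, the spawned room is destroyed and the Gate reopens for the next approach.
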(event Custom|PlayerLocation
  (bind _returnvalue (Game|Player|GetPlayerPawn 0))
  (bind _defaultsceneroot (Variables|Default|GetDefaultSceneRoot))
  (bind _returnvalue_2 (Transformation|GetWorldLocation _defaultsceneroot))
  (bind _rootcomponent (Variables|/Script/Engine.Actor|GetRootComponent _returnvalue))
  (bind _returnvalue_3 (Transformation|GetWorldLocation _rootcomponent))
  (bind _returnvalue_4 (Math|Vector|Distance(Vector) _returnvalue_3 _returnvalue_2))
  (if (< _returnvalue_4 (* 4096.0 3.0))
    (Utilities|FlowControl|Gate false :!label _label
      (:Exit
        (bind _returnvalue_5 (Game|SpawnActorfromClass "/Game/Furniture/Rooms/Mesh/BP_RandomRoom_signs.BP_RandomRoom_Signs_C" (Math|Transform|MakeTransform _returnvalue_2 (Math|Rotator|MakeRotator 0.0 0.0 (Math|Conversions|ToFloat(Integer) (* 90 (Math|Random|RandomIntegerinRange 0 3)))) "1,1,1") "Undefined" 0 0))
        (goto _label Close)))
    (elif (> _returnvalue_4 (* 4096.0 2.0))
      (if (Utilities|IsValid _returnvalue_5)
        (Actor|DestroyActor _returnvalue_5)
        (goto _label Open)))))

(event Custom|BeginPlayerPosition
  (Utilities|Time|SetTimerbyEvent (delegate Custom|PlayerLocation) 1.0 true))

(event EventBeginPlay
  (CallFunction|BeginPlayerPosition))

(event Collision|EventActorBeginOverlap
  (params (OtherActor :type Actor%20Object%20Reference)))

(event EventTick
  (params (DeltaSeconds :type Float%20%28single-precision%29)))

(fn ConstructionScript)