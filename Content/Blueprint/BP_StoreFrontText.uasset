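; Storefront sign actor that randomizes its Text3D name and style at BeginPlay.
; The name usually comes from DT_TextOnly, occasionally from DT_TextStoreFrontDataTable.
; GetDataTable picks a random row of the latter on each call, so font and front material are mixed from independent rows.
; Kerning and word spacing are also randomized, while the bevel and extrude styling is disconnected and never runs.
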(event EventBeginPlay
  (if (> (Math|Random|RandomFloat) 0.15)
    ;[1 1 1] Text
    (bind _outrownames (DataTable|GetDataTableRowNames "/Game/Blueprint/DT_TextOnly.DT_TextOnly"))
    (bind _returnvalue (Utilities|GetDataTableRow "/Game/Blueprint/DT_TextOnly.DT_TextOnly" (.OutItem (Utilities|Array|Random _outrownames)))
      (:then
        (Class|Text3DComponent|SetText (Variables|Default|GetText3D) (Utilities|Struct|BreakTextOnlyStruct _returnvalue))))
    (else
      (bind _storename (CallFunction|GetDataTable))
      (Class|Text3DComponent|SetText (Variables|Default|GetText3D) _storename)))
  (bind _font (CallFunction|GetDataTable))
  (Class|Text3DComponent|SetFont (Variables|Default|GetText3D) _font)
  ;[1 1 1] mics
  (bind _matfront (CallFunction|GetDataTable))
  (Class|Text3DComponent|SetFrontMaterial (Variables|Default|GetText3D) _matfront)
  ;[1 1 1] Kerning
  (Class|Text3DComponent|SetKerning (Variables|Default|GetText3D) (Math|Random|RandomFloatinRange -4.0 15.0))
  (Class|Text3DComponent|SetWordSpacing (Variables|Default|GetText3D) (Math|Random|RandomFloatinRange -2e+01 25.0)))

(event Collision|EventActorBeginOverlap
  (params (OtherActor :type Actor%20Object%20Reference)))

(event EventTick
  (params (DeltaSeconds :type Float%20%28single-precision%29)))

(event Input|KeyboardEvents|SpaceBar
  (params (Key :type Key%20Structure :default "None")))

(event Input|MouseEvents|LeftMouseButton
  (params (Key :type Key%20Structure :default "None")))

(fn ConstructionScript)

(fn GetDataTable
  (bind _outrownames (DataTable|GetDataTableRowNames "/Game/Blueprint/DT_TextStoreFrontDataTable.DT_TextStoreFrontDataTable"))
  (bind _returnvalue (Utilities|GetDataTableRow "/Game/Blueprint/DT_TextStoreFrontDataTable.DT_TextStoreFrontDataTable" (.OutItem (Utilities|Array|Random _outrownames)))
    (:then
      (return (.StoreName (Utilities|Struct|BreakTextDataTableStruct _returnvalue)) (.Font (Utilities|Struct|BreakTextDataTableStruct _returnvalue)) (.MatFront (Utilities|Struct|BreakTextDataTableStruct _returnvalue)) (.MatBevel (Utilities|Struct|BreakTextDataTableStruct _returnvalue)) (.MatExtrude (Utilities|Struct|BreakTextDataTableStruct _returnvalue))))))