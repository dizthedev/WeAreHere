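; BP_Text2D is a text actor that shows a random store name in a random color when play begins.
; BeginPlay usually draws the name from a random DT_TextOnly row, occasionally from DT_TextStoreFrontDataTable through the GetDataTable helper.
; Either path sets the TextRender text, then gives it a random opaque RGB color.
; Unconnected nodes for fonts, materials, bevel and kerning remain in the graph but never run.
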(event EventBeginPlay
  (if (> (Math|Random|RandomFloat) 0.15)
    ;[1 1 1] Text
    (bind _outrownames (DataTable|GetDataTableRowNames "/Game/Blueprint/DT_TextOnly.DT_TextOnly"))
    (bind _returnvalue (Utilities|GetDataTableRow "/Game/Blueprint/DT_TextOnly.DT_TextOnly" (.OutItem (Utilities|Array|Random _outrownames)))
      (:then
        (Rendering|Components|TextRender|SetText (Variables|Default|GetTextRender) (Utilities|Struct|BreakTextOnlyStruct _returnvalue))))
    (else
      (bind _storename (CallFunction|GetDataTable))
      (Rendering|Components|TextRender|SetText (Variables|Default|GetTextRender) _storename)))
  (Rendering|Components|TextRender|SetTextRenderColor (Variables|Default|GetTextRender) (Math|Color|MakeColor (Math|Conversions|ToByte(Integer) (Math|Random|RandomInteger 255)) (Math|Conversions|ToByte(Integer) (Math|Random|RandomInteger 255)) (Math|Conversions|ToByte(Integer) (Math|Random|RandomInteger 255)) 255)))

(event Collision|EventActorBeginOverlap
  (params (OtherActor :type Actor%20Object%20Reference)))

(event EventTick
  (params (DeltaSeconds :type Float%20%28single-precision%29)))

(event Input|KeyboardEvents|SpaceBar
  (params (Key :type Key%20Structure)))

(event Input|MouseEvents|LeftMouseButton
  (params (Key :type Key%20Structure)))

(fn ConstructionScript)

(fn GetDataTable
  (bind _outrownames (DataTable|GetDataTableRowNames "/Game/Blueprint/DT_TextStoreFrontDataTable.DT_TextStoreFrontDataTable"))
  (bind _returnvalue (Utilities|GetDataTableRow "/Game/Blueprint/DT_TextStoreFrontDataTable.DT_TextStoreFrontDataTable" (.OutItem (Utilities|Array|Random _outrownames)))
    (:then
      (return (.StoreName (Utilities|Struct|BreakTextDataTableStruct _returnvalue)) (.Font (Utilities|Struct|BreakTextDataTableStruct _returnvalue)) (.MatFront (Utilities|Struct|BreakTextDataTableStruct _returnvalue)) (.MatBevel (Utilities|Struct|BreakTextDataTableStruct _returnvalue)) (.MatExtrude (Utilities|Struct|BreakTextDataTableStruct _returnvalue))))))